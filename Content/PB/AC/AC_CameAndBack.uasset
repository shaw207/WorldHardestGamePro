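; AC_CameAndBack is an actor component that moves its owning actor back and forth.
; Each tick it offsets the owner in local space by Velocity and Direction scaled by delta time, without sweeping for collisions.
; A looping timer started at BeginPlay negates Direction every Time seconds to reverse the movement.
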(event Custom|OnTimerEnds
  (Variables|Default|SetDirection (* (Variables|Default|GetDirection) -1.0)))

(event EventBeginPlay
  (Utilities|Time|SetTimerbyEvent (delegate Custom|OnTimerEnds) (Variables|Default|GetTime) true))

(event EventTick
  (params (DeltaSeconds :type Float%20%28single-precision%29))
  (Transformation|AddActorLocalOffset (Components|GetOwner) (* DeltaSeconds (Variables|Default|GetVelocity) (Variables|Default|GetDirection)) false false))