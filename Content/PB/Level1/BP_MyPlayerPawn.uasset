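; BP_MyPlayerPawn is the Level 1 player pawn, a Cube pushed around the horizontal plane by player input.
; MyInputAction applies its X/Y value, scaled by Speed, to the Cube as an acceleration-based force.
; BeginPlay puts a score widget on screen without storing a reference, as that assignment is unwired.
; AddScore and Death pass score gains and player death to BP_GameInstance's Level 1 score and death handling.
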(event Input|EnhancedActionEvents|EnhancedInputActionMyInputAction
  (params (ActionValue :type Vector%202D%20Structure) (ElapsedSeconds :type Float%20%28double-precision%29) (TriggeredSeconds :type Float%20%28double-precision%29) (InputAction :type Input%20Action%20Object%20Reference :default "/Game/PB/Level1/Input/MyInputAction.MyInputAction"))
  (bind (_x _y) (Math|Vector2D|BreakVector2D ActionValue))
  (Physics|AddForce (Variables|Default|GetCube) (* (Math|Vector|MakeVector _x _y 0.0) (Variables|Default|GetSpeed)) "None" true))

(event EventBeginPlay
  (bind _returnvalue (UserInterface|CreateWidget "/Game/PB/BP_ScoreWidget.BP_ScoreWidget_C"))
  (UserInterface|Viewport|AddtoViewport _returnvalue 0))

(event Collision|EventActorBeginOverlap
  (params (OtherActor :type Actor%20Object%20Reference)))

(event EventTick
  (params (DeltaSeconds :type Float%20%28single-precision%29)))

(fn ConstructionScript)

(fn AddScore
  (params (Amount :type Integer))
  (bind _asbp_game_instance (Utilities|Casting|CastToBP_GameInstance (Game|GetGameInstance)))
  (Default|SetScoreLevel1 _asbp_game_instance (+ Amount (Variables|/Game/PB/BP_GameInstance.BP_GameInstance_C|GetScoreLevel1 _asbp_game_instance))))

(fn Death
  (bind _asbp_game_instance (Utilities|Casting|CastToBP_GameInstance (Game|GetGameInstance)))
  (Default|PlayerDeathLevel1 _asbp_game_instance))