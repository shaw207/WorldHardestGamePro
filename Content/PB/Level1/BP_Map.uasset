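; BP_Map is a level map actor that toggles between two fixed orientations when the player triggers MapInputAction.
; It enables input on BeginPlay, and a FlipFlop alternates the target rotation on each press, applied instantly with SetActorRotation.
; Collision on its plane, base and cube components is switched off before the rotation and restored to query and physics right after.
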(event Input|EnhancedActionEvents|EnhancedInputActionMapInputAction
  (params (ActionValue :type Boolean) (ElapsedSeconds :type Float%20%28double-precision%29) (TriggeredSeconds :type Float%20%28double-precision%29) (InputAction :type Input%20Action%20Object%20Reference :default "/Game/PB/Level1/Input/MapInputAction.MapInputAction"))
  (:Started
    (Collision|SetCollisionEnabled (Variables|Default|GetPlane) "NoCollision")
    (Utilities|FlowControl|FlipFlop
      (:A
        (Variables|Default|SetRotacion "0.000000,180.000000,180.000000"))
      (:B
        (Variables|Default|SetRotacion "0, 0, 0")))
    (Transformation|SetActorRotation (Variables|Default|GetRotacion))
    (Collision|SetCollisionEnabled (Variables|Default|GetPlane) "QueryAndPhysics")))

(event EventBeginPlay
  (bind _returnvalue (Class|InputDeviceLibrary|GetPlayerControllerfromInputDevice))
  (Input|EnableInput _returnvalue))

(event Collision|EventActorBeginOverlap
  (params (OtherActor :type Actor%20Object%20Reference)))

(event EventTick
  (params (DeltaSeconds :type Float%20%28single-precision%29)))

(fn ConstructionScript)