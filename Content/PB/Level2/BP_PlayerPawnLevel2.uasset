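; Player pawn for Level 2: a physics-driven sphere that rolls along the Y axis from Enhanced Input.
; Input adds mass-independent force scaled by Speed, only when a 100-unit downward line trace finds ground.
; BeginPlay puts the score widget on screen, though the node storing its reference is unconnected.
; AddScore and Death forward to BP_GameInstance, which holds the Level 2 score and handles player death.
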(event Input|EnhancedActionEvents|EnhancedInputActionInputActionLevel2
  (params (ActionValue :type Float%20%28double-precision%29) (ElapsedSeconds :type Float%20%28double-precision%29) (TriggeredSeconds :type Float%20%28double-precision%29) (InputAction :type Input%20Action%20Object%20Reference :default "/Game/PB/Level2/Input/InputActionLevel2.InputActionLevel2"))
  (bind _returnvalue (Collision|LineTraceByChannel (Transformation|GetActorLocation) (+ (Transformation|GetActorLocation) "0.000000,0.000000,-100.000000") "TraceTypeQuery1" false 0 "None"))
  (Variables|Default|SetOnGround _returnvalue)
  (if (Variables|Default|GetOnGround)
    (Physics|AddForce (Variables|Default|GetSphere) (* (Math|Vector|MakeVector 0.0 ActionValue 0.0) (Variables|Default|GetSpeed)) "None" true)))

(event EventBeginPlay
  (bind _returnvalue (UserInterface|CreateWidget "/Game/PB/BP_ScoreWidget.BP_ScoreWidget_C"))
  (UserInterface|Viewport|AddtoViewport _returnvalue 0))

(event Collision|EventActorBeginOverlap
  (params (OtherActor :type Actor%20Object%20Reference)))

(event EventTick
  (params (DeltaSeconds :type Float%20%28single-precision%29)))

(fn ConstructionScript)

(fn AddScore
  (params (NewParam :type Integer))
  (bind _asbp_game_instance (Utilities|Casting|CastToBP_GameInstance (Game|GetGameInstance)))
  (Default|SetScoreLevel2 _asbp_game_instance (+ (Variables|/Game/PB/BP_GameInstance.BP_GameInstance_C|GetScoreLevel2 _asbp_game_instance) NewParam)))

(fn Death
  (bind _asbp_game_instance (Utilities|Casting|CastToBP_GameInstance (Game|GetGameInstance)))
  (Default|PlayerDeathLevel2 _asbp_game_instance))