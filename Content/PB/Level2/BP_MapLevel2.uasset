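; Level 2 map actor that the player rotates around its roll axis in 90-degree steps.
; Each Level2Map input press steps a wrapping four-state angle index, sets the target roll and signed velocity, and starts a two-second cooldown timer.
; Tick advances the roll at that velocity and snaps to the target once within one frame's step.
; An older nearest-quarter-turn snapping chain remains in the graph but is never executed.
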(event Input|EnhancedActionEvents|EnhancedInputActionInputActionLevel2Map
  (params (ActionValue :type Float%20%28double-precision%29) (ElapsedSeconds :type Float%20%28double-precision%29) (TriggeredSeconds :type Float%20%28double-precision%29) (InputAction :type Input%20Action%20Object%20Reference :default "/Game/PB/Level2/Input/InputActionLevel2Map.InputActionLevel2Map"))
  (:Started
    (if (not (Variables|Default|GetRotationCD))
      (Variables|Default|SetRotationCD true)
      (Utilities|Time|SetTimerbyFunctionName 0 "TimerCD" 2.0)
      (Variables|Default|SetAngleCase (+ (Variables|Default|GetAngleCase) ActionValue))
      (if (> (Variables|Default|GetAngleCase) 3)
        (Variables|Default|SetAngleCase 0)
        (elif (< (Variables|Default|GetAngleCase) 0)
          (Variables|Default|SetAngleCase 3)))
      (switch int (Variables|Default|GetAngleCase)
        (:0
          (Variables|Default|SetTargetRotation 0.0))
        (:1
          (Variables|Default|SetTargetRotation 9e+01))
        (:2
          (Variables|Default|SetTargetRotation 1.8e+02))
        (:3
          (Variables|Default|SetTargetRotation -9e+01)))
      (Variables|Default|SetVelocity (* ActionValue (Variables|Default|GetRotationSpeed))))))

(event EventBeginPlay
  (bind _returnvalue (Class|InputDeviceLibrary|GetPlayerControllerfromInputDevice))
  (Input|EnableInput _returnvalue))

(event Collision|EventActorBeginOverlap
  (params (OtherActor :type Actor%20Object%20Reference)))

(event EventTick
  (params (DeltaSeconds :type Float%20%28single-precision%29))
  (Variables|Default|SetCurrentRotation (.Roll (Math|Rotator|BreakRotator (Transformation|GetActorRotation))))
  (if (<= (Math|Float|Absolute(Float) (+ (Variables|Default|GetTargetRotation) (* (Variables|Default|GetCurrentRotation) -1.0))) (* (Variables|Default|GetRotationSpeed) DeltaSeconds))
    (Transformation|SetActorRotation (Math|Rotator|MakeRotator (Variables|Default|GetTargetRotation) 0.0 0.0))
    (else
      (Transformation|SetActorRotation (Math|Rotator|MakeRotator (+ (Variables|Default|GetCurrentRotation) (* (Variables|Default|GetVelocity) DeltaSeconds)) 0.0 0.0)))))

(fn ConstructionScript)

(fn TimerCD
  (Variables|Default|SetRotationCD false))